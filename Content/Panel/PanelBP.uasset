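; Interactable panel actor that unlocks a referenced door when the player uses it.
; Its box overlap stores the FirstPersonCharacter, shows an "Unlock Door" prompt on that character's StringWidget and enables input; ending overlap reverses this.
; Pressing Interact hides the prompt, then, if DoorReference is valid, sets its IsOpen and marks Interacted.
; With InteractOnce set, a used panel no longer offers the prompt on later overlaps.
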(event `self.Box.OnComponentBeginOverlap`
  (params (OverlappedComponent :type "PrimitiveComponent Object Reference") (OtherActor :type "Actor Object Reference") (OtherComp :type "PrimitiveComponent Object Reference") (OtherBodyIndex :type Integer) (bFromSweep :type Boolean) (SweepResult :type "HitResult Structure (by ref)"))
  (if (not (and (`self.Interacted`) (`self.InteractOnce`)))
    (bind _asfirst_person_character (cast `/Game/FirstPersonBP/Blueprints/FirstPersonCharacter` OtherActor))
    (set `self.player` _asfirst_person_character)
    (`/Game/FirstPersonBP/Blueprints/StringWidget.ShowText` (`/Game/FirstPersonBP/Blueprints/FirstPersonCharacter.StringWidget` _asfirst_person_character) true "Unlock Door")
    (`self.EnableInput` (`GameplayStatics.GetPlayerController` 0))))

(event `self.ReceiveActorEndOverlap`
  (params (OtherActor :type "Actor Object Reference"))
  (bind _asfirst_person_character (cast `/Game/FirstPersonBP/Blueprints/FirstPersonCharacter` OtherActor))
  (set `self.player` null)
  (`/Game/FirstPersonBP/Blueprints/StringWidget.HideText` (`/Game/FirstPersonBP/Blueprints/FirstPersonCharacter.StringWidget` _asfirst_person_character))
  (`self.DisableInput` null))

(event `InputAction|Interact`
  (params (Key :type "Key Structure"))
  (bind _doorreference (`self.DoorReference`))
  (:`Pressed`
    (`/Game/FirstPersonBP/Blueprints/StringWidget.HideText` (`/Game/FirstPersonBP/Blueprints/FirstPersonCharacter.StringWidget` (`self.player`)))
    (`/Engine/EditorBlueprintResources/StandardMacros.IsValid` _doorreference
      (:`Is Valid`
        (set `/Game/Door/DoorBP.isOpen` true _doorreference)
        (set `self.Interacted` true)))))

(fn `UserConstructionScript`)