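; Level exit door that lets the first-person player finish the level when IsOpen is set.
; Box overlap shows "Open" and enables input, or shows "Closed"; ending actor overlap hides the text and disables input.
; Interact plays a timeline that cumulatively adds its value to the door's current Z, then calls FinishLevel on the player after a short delay.
; IsOpen is only read here, acting as an unlock flag.
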(event `OpenDoor`
  (bind (_returnvalue_x _returnvalue_y _returnvalue_z) (`KismetMathLibrary.BreakVector` (`self.K2_GetActorLocation`)))
  (bind (_direction _newtrack_0) (`Timeline|Timeline_0`)
    (:`Update`
      (`self.K2_SetActorLocation` (`KismetMathLibrary.MakeVector` _returnvalue_x _returnvalue_y (+ _newtrack_0 _returnvalue_z))))))

(event `self.Box.OnComponentBeginOverlap`
  (params (OverlappedComponent :type "PrimitiveComponent Object Reference") (OtherActor :type "Actor Object Reference") (OtherComp :type "PrimitiveComponent Object Reference") (OtherBodyIndex :type Integer) (bFromSweep :type Boolean) (SweepResult :type "HitResult Structure (by ref)"))
  (if (`self.isOpen`)
    (bind _asfirst_person_character (cast `/Game/FirstPersonBP/Blueprints/FirstPersonCharacter` OtherActor))
    (set `self.player` _asfirst_person_character)
    (`/Game/FirstPersonBP/Blueprints/StringWidget.ShowText` (`/Game/FirstPersonBP/Blueprints/FirstPersonCharacter.StringWidget` _asfirst_person_character) true "Open")
    (`self.EnableInput` (`GameplayStatics.GetPlayerController` 0))
    (else
      (bind _asfirst_person_character_2 (cast `/Game/FirstPersonBP/Blueprints/FirstPersonCharacter` OtherActor))
      (`/Game/FirstPersonBP/Blueprints/StringWidget.ShowText` (`/Game/FirstPersonBP/Blueprints/FirstPersonCharacter.StringWidget` _asfirst_person_character_2) false "Closed"))))

(event `self.ReceiveActorEndOverlap`
  (params (OtherActor :type "Actor Object Reference"))
  (bind _asfirst_person_character (cast `/Game/FirstPersonBP/Blueprints/FirstPersonCharacter` OtherActor))
  (`/Game/FirstPersonBP/Blueprints/StringWidget.HideText` (`/Game/FirstPersonBP/Blueprints/FirstPersonCharacter.StringWidget` _asfirst_person_character))
  (`self.DisableInput` null))

(event `InputAction|Interact`
  (params (Key :type "Key Structure"))
  (bind _player (`self.player`))
  (:`Pressed`
    (`/Game/FirstPersonBP/Blueprints/StringWidget.HideText` (`/Game/FirstPersonBP/Blueprints/FirstPersonCharacter.StringWidget` _player))
    (if (`self.isOpen`)
      (`self.OpenDoor`)
      (`KismetSystemLibrary.Delay` 1.0)
      (`/Game/FirstPersonBP/Blueprints/FirstPersonCharacter.FinishLevel` _player))))

(fn `UserConstructionScript`)